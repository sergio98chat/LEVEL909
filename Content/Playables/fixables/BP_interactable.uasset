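; Base interactable for fixable points that players repair by holding an action of the matching fix type, earning score on completion.
; Overlap registers the point with ThirdPersonCharacter and toggles the Presence effect.
; Tick lowers DeactivationLevel with repair or extinguisher audio while pressed, recovers it otherwise, and updates a camera-yawed circle-bar widget.
; At zero it locks as fixed, awards the sender score and calls EventModifyCustom, apparently a child override hook.
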(event `eventModifyCustom`
  (`KismetSystemLibrary.PrintString` "IN PARENT" true true (struct :`R` 0.120935 :`B` 0.442708 :`A` 1.0) 210.0))

(event `self.ReceiveActorEndOverlap`
  (params (OtherActor :type "Actor Object Reference"))
  ;[1 1 1] OVERLAP AREA FIXABLE
  (set `self.actorInArea` null)
  (set `self.whoIsSendingAction` null)
  (set `self.isFixing` false)
  (bind _asthird_person_character (cast `/Game/ThirdPersonBP/Blueprints/ThirdPersonCharacter` OtherActor))
  (`/Game/ThirdPersonBP/Blueprints/ThirdPersonCharacter.SetCurrentFixablePoint` _asthird_person_character 0 true self)
  (`ActorComponent.Deactivate` (`self.presence`)))

(event `self.ReceiveActorBeginOverlap`
  (params (OtherActor :type "Actor Object Reference"))
  ;[1 1 1] OVERLAP AREA FIXABLE
  (if (`self.ActorHasTag` OtherActor "player")
    (bind _output_get (set `self.actorInArea` OtherActor))
    (bind _asthird_person_character (cast `/Game/ThirdPersonBP/Blueprints/ThirdPersonCharacter` (`self.actorInArea`)))
    (`/Game/ThirdPersonBP/Blueprints/ThirdPersonCharacter.SetCurrentFixablePoint` _asthird_person_character (`self.orderSequenceNumber`) false self)
    (`ActorComponent.Activate` (`self.presence`) false)))

(event `self.ReceiveTick`
  (params (DeltaSeconds :type "Float (single-precision)"))
  (bind _whoissendingaction (`self.whoIsSendingAction`))
  (bind _widget1_2 (`self.Widget1_2`))
  (bind (_returnvalue_roll _returnvalue_pitch) (`KismetMathLibrary.BreakRotator` (`SceneComponent.K2_GetComponentRotation` _widget1_2)))
  (bind (_returnvalue_roll_2 _returnvalue_pitch_2 _returnvalue_yaw) (`KismetMathLibrary.BreakRotator` (`KismetMathLibrary.FindLookAtRotation` (`self.K2_GetActorLocation` (`GameplayStatics.GetPlayerCharacter` 0)) (`PlayerCameraManager.GetCameraLocation` (`PlayerController.PlayerCameraManager` (`GameplayStatics.GetPlayerController` 0))))))
  (`|ExecutionSequence`
    (:`then_0`
      (if (`self.isFixed`)
        _
        (elif (`self.isFixing`)
          ;[1 1 1] FIXATION
          (if (`self.actorIsPressing`)
            (if (not (`self.sound_playing`))
              (if (`|EnumEquality` (`self.typeFix`) "NewEnumerator0")
                (`AudioComponent.Play` (`self.Metal_repair`) 0.0)
                (else
                  (`AudioComponent.Play` (`self.Fire_extinguisher`) 0.0)))
              (set `self.sound_playing` true))
            (bind _output_get (set `self.deactivationLevel` (`KismetMathLibrary.FClamp` (- (`self.deactivationLevel`) (`self.deactivationRate`)) 0.0 100.0)))
            ;[1 1 1] FINAL FIXATION
            (bind _asui_circle_bar_2 (cast `/Game/Playables/fixables/UI_circleBar_2` (`WidgetComponent.GetWidget` (`self.Widget1_2`))))
            (bind _output_get_2 (set `/Game/Playables/fixables/UI_circleBar_2.fixLevel` (`KismetMathLibrary.FCeil` _output_get) _asui_circle_bar_2))
            (if (<= _output_get_2 0)
              (set `self.isFixed` true)
              (`/Engine/EditorBlueprintResources/StandardMacros.IsValid` _whoissendingaction
                (:`Is Valid`
                  (bind _asthird_person_character (cast `/Game/ThirdPersonBP/Blueprints/ThirdPersonCharacter` _whoissendingaction))
                  (`/Game/ThirdPersonBP/Blueprints/ThirdPersonCharacter.AddScore` _asthird_person_character (`self.scoreOfThisPoint`))
                  (`self.eventModifyCustom`)
                  (`AudioComponent.Stop` (`self.Fire_extinguisher`))
                  (`AudioComponent.Stop` (`self.Metal_repair`)))
                (:`Is Not Valid`
                  (`KismetSystemLibrary.PrintString` "NOT VALID")))))
          (else
            (`AudioComponent.Stop` (`self.Metal_repair`))
            (`AudioComponent.Stop` (`self.Fire_extinguisher`))
            (set `self.sound_playing` false)
            ;[1 1 1] AUTO RECOVER BAD FIX
            (`KismetSystemLibrary.Delay` 0.3)
            (bind _output_get_3 (set `self.deactivationLevel` (`KismetMathLibrary.FClamp` (+ (`self.deactivationLevel`) (`self.recoverRate`)) 0.0 100.0)))
            (bind _asui_circle_bar_2_2 (cast `/Game/Playables/fixables/UI_circleBar_2` (`WidgetComponent.GetWidget` (`self.Widget1_2`))))
            (set `/Game/Playables/fixables/UI_circleBar_2.fixLevel` (`KismetMathLibrary.FCeil` _output_get_3) _asui_circle_bar_2_2)))))
    (:`then_1`
      ;[1 1 1] UI ROTATION TO THE CAMERA
      (`SceneComponent.K2_SetWorldRotation` _widget1_2 (`KismetMathLibrary.MakeRotator` _returnvalue_roll _returnvalue_pitch _returnvalue_yaw) false false))))

(event `self.ReceiveBeginPlay`
  (bind _presence (`self.presence`))
  (`ActorComponent.Activate` _presence false)
  (`ActorComponent.Deactivate` _presence)
  (`KismetSystemLibrary.Delay` 0.2))

(event `SetIsFixing`
  (params (actor :type "Actor Object Reference"))
  ;[1 1 1] EVENT SET FIX and PRESS
)

(event `SetActorPressing`
  (params (isPressing :type Boolean) (actorIn :type "Actor Object Reference") (fixTypePlayerIn :type "/Game/Playables/fixables/Enum_typeFix Enum" :default "NewEnumerator0"))
  ;[1 1 1] EVENT SET FIX and PRESS
  (if (`|EnumEquality` fixTypePlayerIn (`self.typeFix`))
    (bind _output_get (set `self.actorIsPressing` isPressing))
    (set `self.isFixing` isPressing)
    (set `self.whoIsSendingAction` actorIn)))

(fn `UserConstructionScript`)