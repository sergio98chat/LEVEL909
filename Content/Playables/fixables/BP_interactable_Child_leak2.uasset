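; A fixable gas leak interactable, a child Blueprint that starts with its AidBand patch hidden.
; Its EventModifyCustom event hides the CascadeGasLeak effect and shows the band.
; It then searches all BP_cloudSpawner actors and disables clouds on those whose association number matches its AssociateCloudSpawner value.
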(event `self.ReceiveBeginPlay`
  (`parent.ReceiveBeginPlay`)
  (`SceneComponent.SetVisibility` (`self.aidBand`) false false))

(event `self.eventModifyCustom`
  (`SceneComponent.SetVisibility` (`self.cascadeGasLeak`) false false)
  (`SceneComponent.SetVisibility` (`self.aidBand`) true false)
  (bind _outactors (`GameplayStatics.GetAllActorsOfClass` "/Game/Cloud/BP_cloudSpawner.BP_cloudSpawner_C"))
  (for _array_element _outactors
    (bind _asbp_cloud_spawner (cast `/Game/Cloud/BP_cloudSpawner` _array_element))
    (if (== (`self.associateCloudSpawner`) (`/Game/Cloud/BP_cloudSpawner.numForAssociate` _asbp_cloud_spawner))
      (set `/Game/Cloud/BP_cloudSpawner.isEnableClouds` false _asbp_cloud_spawner))))

(fn `UserConstructionScript`
  (`parent.UserConstructionScript`))