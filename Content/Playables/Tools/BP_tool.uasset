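; Tool actor that registers when the player is inside its overlap area and shows a world-space bubble icon.
; Begin and end overlap with a player-tagged ThirdPersonCharacter set IsPlayerInTool and notify the character through SetIsInTool, passing itself on entry.
; Tick yaws the icon along the player-to-camera direction, keeping its pitch and roll.
; SetUIToolIconVisibility lets callers show or hide the icon.
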(event `SetUIToolIconVisibility`
  (params (visIn :type Boolean :default true))
  ;[1 1 1] set visibility icon
  (`SceneComponent.SetVisibility` (`self.ui_bubbleToolIcon`) visIn false))

(event `self.ReceiveTick`
  (params (DeltaSeconds :type "Float (single-precision)"))
  (bind _ui_bubbletoolicon (`self.ui_bubbleToolIcon`))
  (bind (_returnvalue_roll _returnvalue_pitch) (`KismetMathLibrary.BreakRotator` (`SceneComponent.K2_GetComponentRotation` _ui_bubbletoolicon)))
  (bind (_returnvalue_roll_2 _returnvalue_pitch_2 _returnvalue_yaw) (`KismetMathLibrary.BreakRotator` (`KismetMathLibrary.FindLookAtRotation` (`self.K2_GetActorLocation` (`GameplayStatics.GetPlayerCharacter` 0)) (`PlayerCameraManager.GetCameraLocation` (`PlayerController.PlayerCameraManager` (`GameplayStatics.GetPlayerController` 0))))))
  ;[1 1 1] icon face rotation
  (`SceneComponent.K2_SetWorldRotation` _ui_bubbletoolicon (`KismetMathLibrary.MakeRotator` _returnvalue_roll _returnvalue_pitch _returnvalue_yaw) false false))

(event `self.ReceiveActorBeginOverlap`
  (params (OtherActor :type "Actor Object Reference"))
  ;[1 1 1] Set player in tool
  (if (`self.ActorHasTag` OtherActor "player")
    (bind _asthird_person_character (cast `/Game/ThirdPersonBP/Blueprints/ThirdPersonCharacter` OtherActor))
    (`/Game/ThirdPersonBP/Blueprints/ThirdPersonCharacter.SetIsInTool` _asthird_person_character true self)
    (set `self.isPlayerInTool` true)))

(event `self.ReceiveActorEndOverlap`
  (params (OtherActor :type "Actor Object Reference"))
  ;[1 1 1] Set player in tool
  (if (`self.ActorHasTag` OtherActor "player")
    (bind _asthird_person_character (cast `/Game/ThirdPersonBP/Blueprints/ThirdPersonCharacter` OtherActor))
    (`/Game/ThirdPersonBP/Blueprints/ThirdPersonCharacter.SetIsInTool` _asthird_person_character false null)
    (set `self.isPlayerInTool` false)))

(fn `UserConstructionScript`)