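; BP_cameraWorld is a fixed camera actor with a trigger box that becomes the player's view and turns to follow the ThirdPersonCharacter.
; Box overlap, or BeginPlay after a short delay, blends the view target to the first BP_cameraWorld in the level, not explicitly itself.
; Tick aims the actor from its CineCamera at the character's capsule, using a reference captured only by that delayed BeginPlay overlap check.
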(event `self.ReceiveTick`
  (params (DeltaSeconds :type "Float (single-precision)"))
  (bind _maincharacter (`self.mainCharacter`))
  (`/Engine/EditorBlueprintResources/StandardMacros.IsValid` _maincharacter
    (:`Is Valid`
      (bind _asthird_person_character (cast `/Game/ThirdPersonBP/Blueprints/ThirdPersonCharacter` _maincharacter))
      (`self.K2_SetActorRotation` (`KismetMathLibrary.FindLookAtRotation` (`SceneComponent.K2_GetComponentLocation` (`self.CineCamera`)) (`SceneComponent.K2_GetComponentLocation` (`Character.CapsuleComponent` _asthird_person_character)))))))

(event `self.Box.OnComponentBeginOverlap`
  (params (OverlappedComponent :type "PrimitiveComponent Object Reference") (OtherActor :type "Actor Object Reference") (OtherComp :type "PrimitiveComponent Object Reference") (OtherBodyIndex :type Integer) (bFromSweep :type Boolean) (SweepResult :type "HitResult Structure (by ref)"))
  ;[1 1 1] Smooth transition to fixed camera
  (bind _asthird_person_character (cast `/Game/ThirdPersonBP/Blueprints/ThirdPersonCharacter` (`|GetArrayItem` (`PrimitiveComponent.GetOverlappingActors` (`self.Box`) "/Game/ThirdPersonBP/Blueprints/ThirdPersonCharacter.ThirdPersonCharacter_C")) :!label _label))
  (`/Engine/EditorBlueprintResources/StandardMacros.IsValid` _asthird_person_character
    (:`Is Valid`
      (bind _asplayer_controller (cast `PlayerController` (`Pawn.GetController` _asthird_person_character)))
      (`/Engine/EditorBlueprintResources/StandardMacros.IsValid` _asplayer_controller
        (:`Is Valid`
          (bind _returnvalue (`GameplayStatics.GetActorOfClass` "BP_cameraWorld_C"))
          (`PlayerController.SetViewTargetWithBlend` _asplayer_controller _returnvalue (`self.blendTime`) "VTBlend_Linear" 0.0 false))))))

(event `self.ReceiveBeginPlay`
  ;[1 1 1] Smooth transition to fixed camera
  (`KismetSystemLibrary.Delay` 1.0)
  (set `self.mainCharacter` (`|GetArrayItem` (`PrimitiveComponent.GetOverlappingActors` (`self.Box`) "/Game/ThirdPersonBP/Blueprints/ThirdPersonCharacter.ThirdPersonCharacter_C")))
  (goto _label))

(fn `UserConstructionScript`)