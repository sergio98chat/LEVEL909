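; BP_Cloud is a hazard cloud that damages actors tagged "player" on capsule overlap and can be blown away by wind.
; Its Plane component gets a very light mass on BeginPlay, so receiveWind pushes it with a scaled impulse.
; After a short random delay it spawns a BP_cloudExplosion at the Plane and hides its skeletal mesh, then destroys both the explosion and itself shortly afterwards.
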(event `self.ReceiveBeginPlay`
  (`PrimitiveComponent.SetMassOverrideInKg` (`self.Plane`) "None" 0.1 true))

(event `self.Capsule.OnComponentBeginOverlap`
  (params (OverlappedComponent :type "PrimitiveComponent Object Reference") (OtherActor :type "Actor Object Reference") (OtherComp :type "PrimitiveComponent Object Reference") (OtherBodyIndex :type Integer) (bFromSweep :type Boolean) (SweepResult :type "HitResult Structure (by ref)"))
  (if (`self.ActorHasTag` OtherActor "player")
    (`GameplayStatics.ApplyDamage` OtherActor (`self.defaultDps`))))

(event `receiveWind`
  (params (force :type "Float (double-precision)") (direction :type "Vector Structure"))
  (`PrimitiveComponent.AddImpulse` (`self.Plane`) (* direction (/ force 10.0)) "None" false)
  (`KismetSystemLibrary.Delay` (`KismetMathLibrary.RandomFloatInRange` 1.0 2.0))
  (bind _returnvalue (`|SpawnActorFromClass` "/Game/Cloud/BP_cloudExplosion.BP_cloudExplosion_C" (`SceneComponent.K2_GetComponentToWorld` (`self.Plane`)) "Undefined" "OverrideRootScale" null null))
  (`SceneComponent.SetVisibility` (`self.SkeletalMesh`) false false)
  (`KismetSystemLibrary.Delay` 2.0)
  (`self.K2_DestroyActor` _returnvalue)
  (`self.K2_DestroyActor` self))

(fn `UserConstructionScript`)