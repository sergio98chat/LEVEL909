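; BP_cloudSpawner is a spawner actor that periodically launches BP_Cloud actors from its SpawnPoint while clouds are enabled.
; BeginPlay sets the launch direction from the root toward SpawnPoint, and a Delay on Tick paces the spawning.
; Each cloud gets randomized scale, linear damping and an impulse within a cone, plus an optional damage-per-second override.
; A looping-timer alternative remains in the graph but never runs.
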(event `self.ReceiveBeginPlay`
  (`|ExecutionSequence`
    (:`then_0`
      (set `self.mainSpawnDirection` (`KismetMathLibrary.Normal` (- (`SceneComponent.K2_GetComponentLocation` (`self.spawn point`)) (`SceneComponent.K2_GetComponentLocation` (`self.DefaultSceneRoot`))))))))

(event `self.ReceiveTick`
  (params (DeltaSeconds :type "Float (single-precision)"))
  (bind _clouddps (`self.cloudDps`))
  (if (`self.isEnableClouds`)
    (`KismetSystemLibrary.Delay` (`self.cloudSpawnerTimer`))
    (bind _cloudout (`self.spawnClouds`))
    (bind _skeletalmesh (`/Game/Cloud/BP_Cloud.SkeletalMesh` _cloudout))
    (`SceneComponent.SetWorldScale3D` _skeletalmesh (/ (`SceneComponent.K2_GetComponentScale` _skeletalmesh) (`KismetMathLibrary.RandomFloatInRange` (`self.minDivScale`) (`self.maxDicScale`))))
    (bind _plane (`/Game/Cloud/BP_Cloud.Plane` _cloudout))
    (`PrimitiveComponent.AddImpulse` _plane (* (`KismetMathLibrary.RandomUnitVectorInConeInDegrees` (`self.mainSpawnDirection`) (`self.coneLaunchAperture`)) (`KismetMathLibrary.RandomFloatInRange` (`self.minForceImpulse`) (`self.maxForceImpulse`))) "None" false)
    (`PrimitiveComponent.SetLinearDamping` _plane (`KismetMathLibrary.RandomFloatInRange` (`self.minLinearDamping`) (`self.maxLinearDamping`)))
    (if (> _clouddps 0.0)
      (set `/Game/Cloud/BP_Cloud.defaultDps` _clouddps _cloudout))))

(fn `spawnClouds`
  (returns (cloudOut :type "/Game/Cloud/BP_Cloud Object Reference"))
  (locals (outCloud :type "/Game/Cloud/BP_Cloud Object Reference"))
  (bind _returnvalue (`|SpawnActorFromClass` "/Game/Cloud/BP_Cloud.BP_Cloud_C" (`SceneComponent.K2_GetComponentToWorld` (`self.spawn point`)) "Undefined" "OverrideRootScale" null null))
  (bind _output_get (set `local.outCloud` _returnvalue))
  (return _output_get))

(fn `UserConstructionScript`)