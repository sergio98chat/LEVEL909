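; NPC pawn that wanders by repeatedly picking a random nearby destination.
; On Tick, while not moving, it waits briefly, then runs AI MoveTo toward a random offset from its root.
; The cone around the initial Cube-to-Arrow direction is wide enough to allow any direction.
; IsMoving blocks new moves until success or failure; cube-hiding and random-chance logic are disconnected.
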(event `self.ReceiveBeginPlay`
  (set `self.mainDir` (`KismetMathLibrary.Normal` (- (`SceneComponent.K2_GetComponentLocation` (`self.Arrow`)) (`SceneComponent.K2_GetComponentLocation` (`self.Cube`))))))

(event `self.ReceiveActorBeginOverlap`
  (params (OtherActor :type "Actor Object Reference")))

(event `self.ReceiveTick`
  (params (DeltaSeconds :type "Float (single-precision)"))
  (if (not (`self.isMoving?`))
    (`KismetSystemLibrary.Delay` 0.2)
    (`|AIMoveTo` (`self.FloatingPawnMovement`) self (+ (`SceneComponent.K2_GetComponentLocation` (`self.DefaultSceneRoot`)) (* (`KismetMathLibrary.RandomUnitVectorInConeInDegrees` (`self.mainDir`) 360.0) (`KismetMathLibrary.RandomFloatInRange` 200.0 400.0))) null
      (:`then`
        (set `self.isMoving?` true))
      (:`OnSuccess`
        (set `self.isMoving?` false :!label _label))
      (:`OnFail`
        (goto _label)))))

(fn `UserConstructionScript`)